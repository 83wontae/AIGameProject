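; BP_SplinePathway is an actor that moves its Sphere component along its Spline in a repeating loop.
; On BeginPlay a timeline track drives a Lerp from zero to the spline length, and the world location at that distance positions the sphere each update.
; Each location is also printed as debug output, and the timeline restarts from the start two seconds after finishing.
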(event EventBeginPlay
  (bind _spline (Variables|Default|GetSpline))
  (bind _새_트랙_0 (Timeline|타임라인_0 PlayFromStart)
    (:Update
      (bind _output_get (Variables|Default|SetLocation (Spline|GetLocationatDistanceAlongSpline _spline (Math|Float|Lerp 0.0 (Spline|GetSplineLength _spline) _새_트랙_0) "World")))
      (Development|PrintString (Utilities|String|ToString(Vector) _output_get))
      (Transformation|SetWorldLocation (Variables|Default|GetSphere) _output_get false false))
    (:Finished
      (Utilities|FlowControl|Delay 2.0)
      (Timeline|타임라인_0 PlayFromStart))))

(fn ConstructionScript)