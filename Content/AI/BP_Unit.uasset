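; BP_Unit is an AI unit that arms itself with a weapon and heads for the player.
; On BeginPlay it spawns a BP_Weapon, snaps it to the mesh's right-hand weapon socket and sets Armed on its Swordsman_AnimBP.
; It then issues a single AIMoveTo toward player pawn 0, which only runs if the anim Blueprint cast succeeds.
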(event EventBeginPlay
  (bind _returnvalue (Game|SpawnActorfromClass "/Game/AI/BP_Weapon.BP_Weapon_C" (Math|Transform|MakeTransform "0, 0, 0") "Undefined" 0 0))
  (Transformation|AttachComponentToComponent _returnvalue (Variables|Character|GetMesh) "hand_r_weapon" "SnapToTarget" "SnapToTarget" "SnapToTarget" true)
  (bind _asswordsman_anim_bp (Utilities|Casting|CastToSwordsman_AnimBP (Components|SkeletalMesh|GetAnimInstance (Variables|Character|GetMesh))))
  (Variables|/Game/Characters/Mannequins/Animations/Swordsman_AnimBP.Swordsman_AnimBP_C|SetArmed _asswordsman_anim_bp true)
  (AI|AIMoveTo self "0, 0, 0" (Game|Player|GetPlayerPawn 0) 5.0 false))

(fn ConstructionScript)